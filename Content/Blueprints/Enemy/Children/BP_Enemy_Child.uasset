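; BP_Enemy_Child is a child enemy Blueprint that gives each spawned enemy a random ghost appearance.
; On BeginPlay it runs the parent logic, then shuffles the GhostMeshes array and applies the first entry to the Ghost static mesh.
; Tick and the construction script only call the parent.
; A disconnected node chain that would yaw the ghost relative to the player pawn's position never runs.
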(event EventBeginPlay
  (bind _ghostmeshes (Variables|Default|GetGhostMeshes))
  (|CallParentFunction)
  ;[1 1 1] Random ghost
  (Utilities|Array|Shuffle _ghostmeshes)
  (Components|StaticMesh|SetStaticMesh (Variables|Default|GetGhost) (Utilities|Array|Get(acopy) _ghostmeshes)))

(event EventTick
  (params (DeltaSeconds :type Float%20%28single-precision%29))
  (|CallParentFunction DeltaSeconds))

(fn ConstructionScript
  (|CallParentFunction))