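; Game director actor that turns low player sanity into audio and visual feedback.
; IsSanityOkay sets the music director's rumble volume inversely to sanity and triggers its fade; its out-of-sanity branch does nothing.
; Tick watches BP_Player's sanity ratio, using paired DoOnce gates to play a timeline below ten percent and reverse it on recovery.
; That timeline fades LUT intensity on the dark post-process volume found at BeginPlay.
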(event Custom|IsSanityOkay
  (params (SanityLevel :type Float%20%28single-precision%29) (SanityMax :type Float%20%28single-precision%29))
  (bind _musicdirectorref (Variables|Default|GetMusicDirectorRef))
  (Utilities|FlowControl|Sequence
    (:then_0
      (bind _output_get (Variables|Default|SetHasRunOutOfSanity (< SanityLevel 0.0)))
      (if _output_get
        _))
    (:then_1
      (Variables|/Game/Blueprints/Directors/BP_Music_Director.BP_Music_Director_C|SetSanityRumbleVolume _musicdirectorref (+ (* (/ SanityLevel SanityMax) -1.0) 1.0))
      (Default|SanityVolumeFade _musicdirectorref))))

(event Custom|PlayStartFade
  (bind _newtrack_0 (Timeline|Timeline_0 PlayFromStart)
    (:Update
      (Variables|/Script/Engine.PostProcessVolume|SetSettings (Variables|Default|GetDarkPProcess) (Utilities|Struct|MakePostProcessSettings _newtrack_0 "/Game/Art/texture/A_LUT_Dark4.A_LUT_Dark4")))))

(event Custom|PLayEndFade
  (bind _newtrack_0 (Timeline|Timeline_0 Reverse)
    (:Update
      (Variables|/Script/Engine.PostProcessVolume|SetSettings (Variables|Default|GetDarkPProcess) (Utilities|Struct|MakePostProcessSettings _newtrack_0 "/Game/Art/texture/A_LUT_Dark4.A_LUT_Dark4")))))

(event EventBeginPlay
  (Utilities|FlowControl|Sequence
    (:then_0
      (bind _outactors (Actor|GetAllActorsOfClass "/Game/Blueprints/Directors/BP_Music_Director.BP_Music_Director_C"))
      (Variables|Default|SetMusicDirectorRef (Utilities|Array|Get(acopy) _outactors)))
    (:then_1
      (bind _outactors_2 (Actor|GetAllActorsOfClass "/Script/Engine.PostProcessVolume"))
      (for _array_element _outactors_2
        (if (== (Utilities|Struct|BreakPostProcessSettings (Variables|/Script/Engine.PostProcessVolume|GetSettings _array_element)) "/Game/Art/texture/A_LUT_Dark4.A_LUT_Dark4")
          (Variables|Default|SetDarkPProcess _array_element))))))

(event EventTick
  (params (DeltaSeconds :type Float%20%28single-precision%29))
  (bind _asbp_player (Utilities|Casting|CastToBP_Player (Game|Player|GetPlayerPawn 0)))
  (if (< (/ (Variables|/Game/Blueprints/PLayer/BP_Player.BP_Player_C|GetCurrentSanityLevel _asbp_player) (Variables|/Game/Blueprints/PLayer/BP_Player.BP_Player_C|GetSanityCap _asbp_player)) 0.1)
    (Utilities|FlowControl|DoOnce false :!label _label
      (:Completed
        (CallFunction|PlayStartFade)
        (goto _label_2 Reset)))
    (else
      (Utilities|FlowControl|DoOnce true :!label _label_2
        (:Completed
          (CallFunction|PLayEndFade)
          (goto _label Reset))))))

(fn ConstructionScript)