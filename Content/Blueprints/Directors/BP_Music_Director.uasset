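; BP_Music_Director is a music director Blueprint that starts the game's soundtrack and a sanity rumble drone on BeginPlay.
; The Insomnia soundtrack loop plays as a fire-and-forget 2D sound, while the drone is a stored 2D audio component with auto-destroy off.
; SanityVolumeFade logarithmically fades that drone to the SanityRumbleVolume variable, and is called here once, right after the drone starts.
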(event Custom|MainMusic
  (Audio|PlaySound2D "/Game/Audio/Insomnia_Soundtrack_Loop.Insomnia_Soundtrack_Loop" 1.0 1.0 0.0 0 0))

(event Custom|SanityRumbleDrone
  (bind _returnvalue (Audio|CreateSound2D "/Game/Audio/Drones/CUE_SanityLowing.CUE_SanityLowing" 1.2 1.0 0.0 0 false false))
  (bind _output_get (Variables|Default|SetSanityRumble _returnvalue))
  (Audio|Components|Audio|Play _output_get 0.0)
  (CallFunction|SanityVolumeFade))

(event Custom|SanityVolumeFade
  (Audio|Components|Audio|AdjustVolume (Variables|Default|GetSanityRumble) 1.0 (Variables|Default|GetSanityRumbleVolume) "Logarithmic" :!class /Script/Engine.AudioComponent))

(event EventBeginPlay
  (CallFunction|MainMusic)
  (CallFunction|SanityRumbleDrone))

(event Collision|EventActorBeginOverlap
  (params (OtherActor :type Actor%20Object%20Reference)))

(event EventTick
  (params (DeltaSeconds :type Float%20%28single-precision%29)))

(fn ConstructionScript)