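; BP_AI_CandleDirector is a director actor that keeps a list of the level's candles that are available, presumably for AI use.
; On BeginPlay, StoreAvailableCandles gathers every BP_Candle into AllCandles and rebuilds AllAvailableCandles from those that are lit and not flagged InValidCandle.
; The list refreshes only when that event is called; Tick just logs its count each frame as debug output.
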(event Custom|StoreAvailableCandles
  (Utilities|Array|Clear (Variables|Default|GetAllAvailableCandles))
  (bind _outactors (Actor|GetAllActorsOfClass "/Game/Blueprints/Candle/BP_Candle.BP_Candle_C"))
  (bind _output_get (Variables|Default|SetAllCandles _outactors))
  (for _array_element _output_get
    (if (not (Variables|/Game/Blueprints/Candle/BP_Candle.BP_Candle_C|GetInValidCandle _array_element))
      (if (Variables|/Game/Blueprints/Candle/BP_Candle.BP_Candle_C|GetIsLit _array_element)
        (Utilities|Array|Add (Variables|Default|GetAllAvailableCandles) _array_element)))))

(event EventBeginPlay
  (CallFunction|StoreAvailableCandles))

(event Collision|EventActorBeginOverlap
  (params (OtherActor :type Actor%20Object%20Reference)))

(event EventTick
  (params (DeltaSeconds :type Float%20%28single-precision%29))
  (Development|PrintString (Utilities|String|ToString(Integer) (Utilities|Array|Length (Variables|Default|GetAllAvailableCandles))) false true "(R=0.000000,G=0.660000,B=1.000000,A=1.000000)" 0.0))

(fn ConstructionScript)