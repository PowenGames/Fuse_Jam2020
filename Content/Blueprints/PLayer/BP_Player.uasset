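; First-person player that carries a candle, throws it and picks it back up, with sanity driven by candlelight.
; BeginPlay spawns the HUD, held candle and darkness sphere.
; Interact throws by hiding the held candle and spawning a projectile copy, or retrieves that copy with its lit state, updating the vision sphere and AI candle director.
; A looping timer line-traces to visible lit candles, adjusting and debug-printing sanity by hit distance.
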(event Custom|UpdateSanity
  (Variables|Sanity|SetSanityIncrease 0.0)
  (for _array_element (Variables|/Game/Blueprints/Directors/BP_AI_CandleDirector.BP_AI_CandleDirector_C|GetAllCandles (Variables|References|GetAICandleDirectorRef))
    (if (and (Variables|/Game/Blueprints/Candle/BP_Candle.BP_Candle_C|GetIsLit _array_element) (not (Variables|/Script/Engine.Actor|GetbHidden _array_element)))
      (bind _outhit (Collision|LineTraceByChannel (Transformation|GetWorldLocation (Variables|Default|GetCamera)) (Transformation|GetActorLocation _array_element) "TraceTypeQuery1" false 0 "ForOneFrame"))
      (if (.bBlockingHit (Collision|BreakHitResult _outhit))
        ;[1 1 1] Seems to default to 90 when moving far away
        (if (< (.Distance (Collision|BreakHitResult _outhit)) (Variables|Sanity|GetLightMinThreshold))
          (Variables|Sanity|SetSanityIncrease (+ (Variables|Sanity|GetSanityIncrease) (Math|Float|Clamp(Float) (* (* (- (.Distance (Collision|BreakHitResult _outhit)) (Variables|Sanity|GetLightMinThreshold)) -1.0) 0.2) 0.0 1e+02)))
          (else
            (Variables|Sanity|SetSanityIncrease (- (Variables|Sanity|GetSanityIncrease) 1e+01)))))))
  (bind _output_get (Variables|Sanity|SetCurrentSanityLevel (+ (Variables|Sanity|GetSanityIncrease) (Variables|Sanity|GetCurrentSanityLevel))))
  (Development|PrintString (Utilities|String|Append "Inc: " (Utilities|String|ToString(Float) (Variables|Sanity|GetSanityIncrease)) " Cur: " (Utilities|String|ToString(Float) _output_get)) true true "(R=0.000000,G=0.660000,B=1.000000,A=1.000000)" 1.0))

(event EventBeginPlay
  (Utilities|FlowControl|Sequence
    (:then_0
      ;[1 1 1] References
      (bind _outactors (Actor|GetAllActorsOfClass "/Game/Blueprints/Directors/BP_AI_CandleDirector.BP_AI_CandleDirector_C"))
      (Variables|References|SetAICandleDirectorRef (Utilities|Array|Get(acopy) _outactors)))
    (:then_1
      ;[1 1 1] Create hud
      (bind _returnvalue (UserInterface|CreateWidget "/Game/Blueprints/UI/WBP_HUD.WBP_HUD_C"))
      (UserInterface|Viewport|AddtoViewport _returnvalue 0))
    (:then_2
      (bind _returnvalue_2 (Game|SpawnActorfromClass "/Game/Blueprints/Candle/BP_Candle.BP_Candle_C" (Math|Transform|MakeTransform "0, 0, 0" "0, 0, 0" "1,1,1") "Undefined" 0 0))
      (bind _output_get (Variables|References|SetAttachedCandle _returnvalue_2))
      (Default|ActivateCandle _output_get false)
      (Transformation|AttachComponentToComponent (Variables|References|GetAttachedCandle) (Variables|Default|GetCandleAttachPoint) "None" "SnapToTarget" "SnapToTarget" "SnapToTarget" false)
      (Variables|/Game/Blueprints/Candle/BP_Candle.BP_Candle_C|SetIsHeld (Variables|References|GetAttachedCandle) true))
    (:then_3
      (bind _returnvalue_3 (Game|SpawnActorfromClass "/Game/Blueprints/Art/BP_DarknessSphere.BP_DarknessSphere_C" (Math|Transform|MakeTransform "0, 0, 0" "0, 0, 0" "1,1,1") "Undefined" 0 0))
      (bind _output_get_2 (Variables|References|SetDarknessSphere _returnvalue_3))
      (Transformation|AttachComponentToComponent _output_get_2 (Variables|Default|GetDarkSphereAttachPoint) "None" "SnapToTarget" "SnapToTarget" "SnapToTarget" false))
    (:then_4
      (bind _returnvalue_4 (Utilities|Time|SetTimerbyFunctionName 0 "UpdateSanity" 0.5 true))
      (Variables|Default|SetSanityTimer _returnvalue_4))))

(event EventTick
  (params (DeltaSeconds :type Float%20%28single-precision%29)))

(event Input|ActionEvents|InputActionInteract
  (params (Key :type Key%20Structure :default "None"))
  (bind _attachedcandle (Variables|References|GetAttachedCandle))
  ;[1 1 1] Interacting and throwing
  (:Pressed
    (if (Variables|/Script/Engine.Actor|GetbHidden (Variables|References|GetAttachedCandle))
      (bind _array_element (Utilities|Array|ForEachLoopwithBreak (Collision|GetOverlappingActors (Variables|Default|GetPickupSphere) "/Game/Blueprints/Candle/BP_Candle.BP_Candle_C" :!class /Script/Engine.PrimitiveComponent) :!label _label)
        (:LoopBody
          (bind _asbp_candle (Utilities|Casting|CastToBP_Candle _array_element))
          (if (not (== (Variables|References|GetAttachedCandle) _asbp_candle))
            (if (== (Variables|References|GetLastCandleThrown) _asbp_candle)
              (Variables|Default|SetPickupCandleLitStatus (Variables|/Game/Blueprints/Candle/BP_Candle.BP_Candle_C|GetIsLit (Variables|References|GetLastCandleThrown)))
              (Actor|DestroyActor (Variables|References|GetLastCandleThrown))
              (Variables|References|SetLastCandleThrown 0)
              (CallFunction|HideCandle false)
              (goto _label Break))))
        (:Completed
          (Utilities|IsValid (Variables|References|GetLastCandleThrown)
            (:Is%20Not%20Valid
              (Default|SpawnCandleLight _attachedcandle)
              (Default|TurnonLight (Variables|/Game/Blueprints/Candle/BP_Candle.BP_Candle_C|GetPointlightRef _attachedcandle) (Variables|Default|GetPickupCandleLitStatus))
              (Default|ReverseShrink (Variables|References|GetDarknessSphere))
              (Default|ActivateCandle _attachedcandle (not (Variables|Default|GetPickupCandleLitStatus)))
              (Variables|/Game/Blueprints/Candle/BP_Candle.BP_Candle_C|SetInValidCandle (Variables|References|GetAttachedCandle) false)
              (Default|StoreAvailableCandles (Variables|References|GetAICandleDirectorRef))))))
      (else
        (Default|ShrinkVision (Variables|References|GetDarknessSphere))
        (bind _returnvalue (Game|SpawnActorfromClass "/Game/Blueprints/Candle/BP_Candle.BP_Candle_C" (Math|Transform|MakeTransform (Transformation|GetWorldLocation (Variables|Default|GetCandleAttachPoint)) (Transformation|GetWorldRotation (Variables|Default|GetCamera)) "1,1,1") "Undefined" 0 0))
        (bind _output_get (Variables|References|SetLastCandleThrown _returnvalue))
        (Default|EnablePhysics _output_get false)
        (Components|Activation|Activate (Variables|/Game/Blueprints/Candle/BP_Candle.BP_Candle_C|GetProjectileMovement (Variables|References|GetLastCandleThrown)) false)
        (Variables|/Game/Blueprints/Candle/BP_Candle.BP_Candle_C|SetProjectileMode (Variables|References|GetLastCandleThrown) true)
        (CallFunction|HideCandle true)
        (Variables|/Game/Blueprints/Candle/BP_Candle.BP_Candle_C|SetInValidCandle (Variables|References|GetAttachedCandle) true)
        (Default|StoreAvailableCandles (Variables|References|GetAICandleDirectorRef))))))

(event Input|AxisEvents|InputAxisForward
  (params (AxisValue :type Float%20%28single-precision%29))
  ;[1 1 1] Movement and Axis
  ;;[1 1 1] Player movement
  (Pawn|Input|AddMovementInput (Math|Vector|GetForwardVector (Transformation|GetActorRotation)) AxisValue false))

(event Input|AxisEvents|InputAxisRight
  (params (AxisValue :type Float%20%28single-precision%29))
  ;[1 1 1] Movement and Axis
  ;;[1 1 1] Player movement
  (Pawn|Input|AddMovementInput (Math|Vector|GetRightVector (Transformation|GetActorRotation)) AxisValue false))

(event Input|AxisEvents|InputAxisMouseYAxis
  (params (AxisValue :type Float%20%28single-precision%29))
  ;[1 1 1] Movement and Axis
  ;;[1 1 1] Mouse movement
  (Pawn|Input|AddControllerPitchInput AxisValue))

(event Input|AxisEvents|InputAxisMouseXAxis
  (params (AxisValue :type Float%20%28single-precision%29))
  ;[1 1 1] Movement and Axis
  ;;[1 1 1] Mouse movement
  (Pawn|Input|AddControllerYawInput AxisValue))

(fn ConstructionScript)

(fn LineTracefromCamera
  (bind _returnvalue (Transformation|GetActorLocation))
  (Collision|LineTraceByChannel _returnvalue (Math|Vector|RotateVector _returnvalue (Transformation|GetWorldRotation (Variables|Default|GetCamera))) "TraceTypeQuery1" false 0 "Persistent"))

(fn HideCandle
  (params (Hidden :type Boolean))
  (bind _attachedcandle (Variables|References|GetAttachedCandle))
  (Rendering|SetActorHiddenInGame _attachedcandle Hidden)
  (if Hidden
    (Default|ActivateCandle _attachedcandle false)
    (Actor|DestroyActor (Variables|/Game/Blueprints/Candle/BP_Candle.BP_Candle_C|GetPointlightRef (Variables|References|GetAttachedCandle)))))